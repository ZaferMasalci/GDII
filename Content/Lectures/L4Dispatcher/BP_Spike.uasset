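; BP_Spike is a spike trap actor that damages the third-person player character.
; When the player overlaps the Activation volume, a timeline animates the Spikes' height, and overlapping the Damage component reduces player health.
; It binds to the character's DPTrapType event dispatcher on BeginPlay, and a matching trap type lowers the spikes and disables damage collision.
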(event `self.ReceiveBeginPlay`
  (bind _asbp_third_person_character (cast `/Game/ThirdPerson/Blueprints/BP_ThirdPersonCharacter` (`GameplayStatics.GetPlayerCharacter` 0)))
  (bind _output_get (set `self.As BP Third Person Character` _asbp_third_person_character))
  (add `/Game/ThirdPerson/Blueprints/BP_ThirdPersonCharacter.DP_TrapType` _output_get (delegate `DP_TrapType_Event`)))

(event `DP_TrapType_Event`
  (params (TrapType :type "/Game/Lectures/L4Dispatcher/E_TrapType Enum" :default "NewEnumerator0"))
  (if (`|EnumEquality` TrapType (`self.TrapType`))
    (`SceneComponent.K2_SetRelativeLocation` (`self.Spikes`) (0.0 0.0 -60.0) false false)
    (`PrimitiveComponent.SetCollisionEnabled` (`self.Damage`) "NoCollision")))

(event `self.Activation.OnComponentBeginOverlap`
  (params (OverlappedComponent :type "PrimitiveComponent Object Reference") (OtherActor :type "Actor Object Reference") (OtherComp :type "PrimitiveComponent Object Reference") (OtherBodyIndex :type Integer) (bFromSweep :type Boolean) (SweepResult :type "HitResult Structure (by ref)"))
  (if (== OtherActor (`self.As BP Third Person Character`))
    (`self.Spikes`
      (:`then`
        (bind (_direction _newtrack_0) (`Timeline|Spike`)
          (:`Update`
            (`SceneComponent.K2_SetRelativeLocation` (`self.Spikes`) (`KismetMathLibrary.MakeVector` 0.0 0.0 _newtrack_0) false false))))
      (:`else`))))

(event `self.Damage.OnComponentBeginOverlap`
  (params (OverlappedComponent :type "PrimitiveComponent Object Reference") (OtherActor :type "Actor Object Reference") (OtherComp :type "PrimitiveComponent Object Reference") (OtherBodyIndex :type Integer) (bFromSweep :type Boolean) (SweepResult :type "HitResult Structure (by ref)"))
  (bind _as_bp_third_person_character (`self.As BP Third Person Character`))
  (if (== OtherActor _as_bp_third_person_character)
    (`/Game/ThirdPerson/Blueprints/BP_ThirdPersonCharacter.HealthUpdate` _as_bp_third_person_character -15.0)))

(fn `UserConstructionScript`)