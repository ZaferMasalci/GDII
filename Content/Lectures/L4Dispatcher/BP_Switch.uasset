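; BP_Switch is an interactable switch that signals traps of its assigned TrapType, with a debug message indicating they turn off.
; On BeginPlay it caches the player's BP_ThirdPersonCharacter and shows the trap type's name on a text render.
; Interact calls the character's DPTrapType event dispatcher with that type, using the player as the broadcast hub rather than referencing traps directly.
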(event `self.ReceiveBeginPlay`
  (bind _asbp_third_person_character (cast `/Game/ThirdPerson/Blueprints/BP_ThirdPersonCharacter` (`GameplayStatics.GetPlayerCharacter` 0)))
  (set `self.As BP Third Person Character` _asbp_third_person_character)
  (`TextRenderComponent.K2_SetText` (`self.TextRender`) (`KismetTextLibrary.Conv_StringToText` (`|GetEnumeratorNameAsString` (`self.TrapType`)))))

(event `/Game/Lectures/L4Dispatcher/BPI_Interactable.Interact`
  (`/Game/ThirdPerson/Blueprints/BP_ThirdPersonCharacter.DP_TrapType` (`self.As BP Third Person Character`) (`self.TrapType`))
  (`KismetSystemLibrary.PrintString` "Turn Off Trap"))

(fn `UserConstructionScript`)