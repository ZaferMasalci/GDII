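; BP_MazeCell is a single maze cell actor that builds its floor and optional North, South, East and West walls in the Construction Script.
; GridSize drives wall length and thickness, which SizeToScale converts from centimetres to mesh scale.
; CreateWall adds a static mesh component for each enabled wall flag, using WallOffset to place the North and East walls on the far edges.
; The event graph holds no runtime logic.
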(fn `UserConstructionScript`
  (bind _gridsize (`self.GridSize`))
  (bind _walllength (`self.WallLength`))
  (bind _walllength_2 (`self.WallLength`))
  (bind _walllength_3 (`self.WallLength`))
  (bind _walllength_4 (`self.WallLength`))
  (bind _walllength_5 (`self.WallLength`))
  (set `self.WallLength` _gridsize)
  (set `self.WallThickness` (* _gridsize 0.1))
  (`SceneComponent.SetRelativeScale3D` (`self.Floor`) (`self.SizeToScale` (`KismetMathLibrary.MakeVector` _walllength_4 _walllength_4 (`self.WallThickness`))))
  (`self.CreateWall` (`self.WestWall`) 0.0 0.0 0.0 (`self.SizeToScale` (`KismetMathLibrary.MakeVector` _walllength_5 (`self.WallThickness`) _walllength_5))
    (:`True`
      _)
    (:`false`
      _))
  (`self.CreateWall` (`self.EastWall`) 0.0 (`self.WallOffset`) 0.0 (`self.SizeToScale` (`KismetMathLibrary.MakeVector` _walllength (`self.WallThickness`) _walllength))
    (:`True`
      _)
    (:`false`
      _))
  (`self.CreateWall` (`self.SouthWall`) 0.0 0.0 0.0 (`self.SizeToScale` (`KismetMathLibrary.MakeVector` (`self.WallThickness`) _walllength_2 _walllength_2))
    (:`True`
      _)
    (:`false`
      _))
  (`self.CreateWall` (`self.NorthWall`) (`self.WallOffset`) 0.0 0.0 (`self.SizeToScale` (`KismetMathLibrary.MakeVector` (`self.WallThickness`) _walllength_3 _walllength_3))))