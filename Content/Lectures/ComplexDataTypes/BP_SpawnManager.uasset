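; BP_SpawnManager is a key-driven enemy spawner and damage tester from the ComplexDataTypes lecture.
; F picks a random enemy type, looks up its difficulty in a map and its stats in DT_EnemyStats using the enum name as row name.
; It then spawns a BP_EnemyBase at a random X/Y with that data and stores it in SpawnEnemies.
; X applies fixed damage to every valid stored enemy.
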(event `self.ReceiveBeginPlay`
  (`self.EnableInput` (`GameplayStatics.GetPlayerController` 0)))

(event `Key|F`
  (params (Key :type "Key Structure"))
  (:`Pressed`
    (bind _output_get (set `self.SpawnedEnemy` (`|GetArrayItem` (`self.EEnemyTypes`) (`KismetMathLibrary.RandomIntegerInRange` 0 3))))
    (set `self.SpawnedDifficulty` (`BlueprintMapLibrary.Map_Find` (`self.EnemyDifficulty`) _output_get))
    (bind _returnvalue (`|GetDataTableRow` "/Game/Lectures/ComplexDataTypes/DT_EnemyStats.DT_EnemyStats" (`KismetStringLibrary.Conv_StringToName` (`|GetEnumeratorNameAsString` _output_get)))
      (:`then`
        (set `self.SpawnedEnemyStats` _returnvalue)
        (bind _returnvalue_2 (`|SpawnActorFromClass` "/Game/Lectures/ComplexDataTypes/BP_EnemyBase.BP_EnemyBase_C" (`KismetMathLibrary.MakeTransform` (`KismetMathLibrary.MakeVector` (`KismetMathLibrary.RandomFloatInRange` 100.0 1000.0) (`KismetMathLibrary.RandomFloatInRange` 100.0 1000.0))) "Undefined" "MultiplyWithRoot" null (`self.SpawnedEnemy`) (`self.SpawnedEnemyStats`) (`self.SpawnedDifficulty`) null))
        (`KismetArrayLibrary.Array_Add` (`self.SpawnEnemies`) _returnvalue_2)))))

(event `Key|X`
  (params (Key :type "Key Structure"))
  (:`Pressed`
    (for _array_element (`self.SpawnEnemies`)
      (`/Engine/EditorBlueprintResources/StandardMacros.IsValid` _array_element
        (:`Is Valid`
          (`/Game/Lectures/ComplexDataTypes/BP_EnemyBase.TakeDamage` _array_element 50.0))))))

(fn `UserConstructionScript`)