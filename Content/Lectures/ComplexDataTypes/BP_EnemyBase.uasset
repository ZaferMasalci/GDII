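; Base enemy Blueprint from a lecture on complex data types, configured through an EnemyType enum and an EnemyStats struct.
; On BeginPlay it copies health, speed and damage from the struct, labels itself with type and health, and picks a skeletal mesh per type.
; Tick slides it along world X by MoveSpeed.
; TakeDamage reduces health and, at zero, destroys the actor and spawns BP_Loot with gold scaled by Difficulty.
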(event `self.ReceiveBeginPlay`
  (bind _mesh (`self.Mesh`))
  (bind (_health _damage _speed) (break `/Game/Lectures/ComplexDataTypes/ST_EnemyStats` (`self.EnemyStats`)))
  (bind _output_get (set `self.CurrentHealth` _health))
  (set `self.MoveSpeed` _speed)
  (set `self.AttackDamage` _damage)
  (`TextRenderComponent.K2_SetText` (`self.TextRender`) (`KismetTextLibrary.Conv_StringToText` (`KismetStringLibrary.Concat_StrStr` (`|GetEnumeratorNameAsString` (`self.EnemyType`)) "/" (`KismetStringLibrary.Conv_DoubleToString` _output_get))))
  (switch `/Game/Lectures/ComplexDataTypes/EEnemyType` (`self.EnemyType`)
    (:`NewEnumerator0`
      (`SkeletalMeshComponent.SetSkeletalMeshAsset` _mesh "/Game/Characters/Mannequins/Meshes/SKM_Manny_Simple.SKM_Manny_Simple"))
    (:`NewEnumerator1`
      (`SkeletalMeshComponent.SetSkeletalMeshAsset` _mesh "/Game/Characters/Mannequins/Meshes/SKM_Manny_Simple1.SKM_Manny_Simple1"))
    (:`NewEnumerator2`
      (`SkeletalMeshComponent.SetSkeletalMeshAsset` _mesh "/Game/Characters/Mannequins/Meshes/SKM_Quinn_Simple.SKM_Quinn_Simple"))
    (:`NewEnumerator3`
      (`SkeletalMeshComponent.SetSkeletalMeshAsset` _mesh "/Game/Characters/Mannequins/Meshes/SKM_Quinn_Simple1.SKM_Quinn_Simple1"))))

(event `self.ReceiveTick`
  (params (DeltaSeconds :type "Float (single-precision)"))
  ; Walk
  (`self.K2_AddActorWorldOffset` (`KismetMathLibrary.MakeVector` (* DeltaSeconds (`self.MoveSpeed`) 50.0))))

(fn `TakeDamage`
  (params (Damage :type "Float (double-precision)"))
  (returns (ReturnValue :type "Float (double-precision)"))
  (bind _output_get (set `self.CurrentHealth` (- (`self.CurrentHealth`) Damage)))
  (if (<= _output_get 0.0)
    (`self.K2_DestroyActor`)
    (`|SpawnActorFromClass` "/Game/Lectures/ComplexDataTypes/BP_Loot.BP_Loot_C" (`self.GetTransform`) "Undefined" "MultiplyWithRoot" null (* (`self.Difficulty`) 100) null)
    (else
      (return _output_get))))

(fn `UserConstructionScript`)